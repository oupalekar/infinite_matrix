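; Health pickup actor that restores a fixed amount of health to the player on contact.
; A Box overlap casts the other actor to BP_Player, adds to its Health within a clamped range, then destroys the pack.
; A PawnInFront event also destroys the pack once the supplied pawn's world X exceeds its own, removing pickups the pawn has passed.
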(event OnComponentBeginOverlap(Box)
  (params (OverlappedComponent :type Primitive%20Component%20Object%20Reference) (OtherActor :type Actor%20Object%20Reference) (OtherComp :type Primitive%20Component%20Object%20Reference) (OtherBodyIndex :type Integer) (bFromSweep :type Boolean) (SweepResult :type Hit%20Result%20Structure%20%28by%20ref%29))
  (Utilities|FlowControl|Sequence
    (:then_0
      (bind _asbp_player (Utilities|Casting|CastToBP_Player OtherActor))
      (Variables|/Game/InfiniteMatrix/Blueprints/BP_Player.BP_Player_C|SetHealth _asbp_player (Math|Float|Clamp(Float) (+ (Variables|/Game/InfiniteMatrix/Blueprints/BP_Player.BP_Player_C|GetHealth _asbp_player) 2e+01) 0.0 1e+02))
      (Actor|DestroyActor))))

(event Custom|Pawn%20In%20Front
  (params (pawn%20position :type BP%20Player%20Object%20Reference))
  (if (> (.x (Transformation|GetActorLocation pawn%20position)) (.x (Transformation|GetActorLocation)))
    (Actor|DestroyActor self)))

(event EventBeginPlay)

(event Collision|EventActorBeginOverlap
  (params (OtherActor :type Actor%20Object%20Reference)))

(event EventTick
  (params (DeltaSeconds :type Float%20%28single-precision%29)))

(fn ConstructionScript)