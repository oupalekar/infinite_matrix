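; Projectile actor that flies along an axis and destroys enemies it hits.
; Tick offsets it along world X by InitialSpeed scaled by delta time.
; On Hit it destroys itself, then destroys Other if it is a BP_Enemy.
; The score increment follows that cast and casts the same Other to BP_Player, so it only runs if Other passes both casts.
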(event EventBeginPlay)

(event Collision|EventActorBeginOverlap
  (params (OtherActor :type Actor%20Object%20Reference)))

(event EventTick
  (params (DeltaSeconds :type Float%20%28single-precision%29))
  (Transformation|AddActorWorldOffset (Math|Vector|MakeVector (* (Variables|Default|GetInitialSpeed) DeltaSeconds) 0.0 0.0)))

(event Collision|EventHit
  (params (MyComp :type Primitive%20Component%20Object%20Reference) (Other :type Actor%20Object%20Reference) (OtherComp :type Primitive%20Component%20Object%20Reference) (bSelfMoved :type Boolean) (HitLocation :type Vector :default "0, 0, 0") (HitNormal :type Vector :default "0, 0, 0") (NormalImpulse :type Vector :default "0, 0, 0") (Hit :type Hit%20Result%20Structure%20%28by%20ref%29))
  (Utilities|FlowControl|Sequence
    (:then_0
      (Actor|DestroyActor))
    (:then_1
      (bind _asbp_enemy (Utilities|Casting|CastToBP_Enemy Other))
      (Actor|DestroyActor _asbp_enemy)
      (bind _asbp_player (Utilities|Casting|CastToBP_Player Other))
      (Variables|/Game/InfiniteMatrix/Blueprints/BP_Player.BP_Player_C|SetScore _asbp_player (+ (Variables|/Game/InfiniteMatrix/Blueprints/BP_Player.BP_Player_C|GetScore _asbp_player) 1)))))

(fn ConstructionScript)